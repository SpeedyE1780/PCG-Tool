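; BP_CombinationActor is an actor that groups four shape entries (sphere, cube, cone and cylinder scenes) into CombinationSet.
; The construction script clears the collection and refills it through the AddItemToCombination helper, so it is rebuilt on each construction.
; The event graph has no active logic, and nothing here reads or uses the collection afterwards.
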(event EventBeginPlay)

(event Collision|EventActorBeginOverlap
  (params (OtherActor :type Actor%20Object%20Reference)))

(event EventTick
  (params (DeltaSeconds :type Float%20%28single-precision%29)))

(fn ConstructionScript
  (Utilities|Array|Clear (Variables|Default|GetcombinationSet))
  (CallFunction|AddItemtoCombination (Variables|Default|GetSphereScene))
  (CallFunction|AddItemtoCombination (Variables|Default|GetCubeScene))
  (CallFunction|AddItemtoCombination (Variables|Default|GetConeScene))
  (CallFunction|AddItemtoCombination (Variables|Default|GetCylinderScene)))

(fn AddItemtoCombination
  (params (Item :type Scene%20Component%20Object%20Reference%20%28by%20ref%29))
  (Utilities|Array|Add (Variables|Default|GetcombinationSet) Item)
  (return))